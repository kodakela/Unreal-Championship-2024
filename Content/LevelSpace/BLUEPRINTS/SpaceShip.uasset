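; SpaceShip is a physics-driven, player-controlled ship Blueprint that moves through forces on its SpaceShip component.
; The Speed axis applies thrust along the component's right vector as an acceleration change, so mass is ignored.
; The LeftRight axis applies torque around the component's up vector to yaw the ship, with mass affecting the turn.
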(event Input|AxisEvents|InputAxisSpeed
  (params (AxisValue :type Float%20%28single-precision%29))
  (Physics|AddForce (Variables|Default|GetSpaceShip) (* (Math|Vector|GetRightVector (Variables|Default|GetSpaceShip)) (* AxisValue 1e+02)) "None" true))

(event Input|AxisEvents|InputAxisLeftRight
  (params (AxisValue :type Float%20%28single-precision%29))
  (Class|PrimitiveComponent|AddTorqueinDegrees (Variables|Default|GetSpaceShip) (* (Math|Vector|GetUpVector (Variables|Default|GetSpaceShip)) (* AxisValue 1e+02)) "None" false))

(fn ConstructionScript)