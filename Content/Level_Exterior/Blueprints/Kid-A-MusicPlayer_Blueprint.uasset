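; Music player Blueprint for the exterior level that plays Radiohead's Kid A album track by track through an audio component.
; SelectNewSong maps an index to title and track, and BeginPlay fades the track in, then re-selects after a Delay of its duration.
; Each selection also stores the title in GI_KidA and calls CallWidget on the first-person character.
; PlaySongNofuncioandelay is an uncalled variant, named as non-working, using submix delay settings.
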(event EventBeginPlay
  (bind (_audiocomponent _selected _nombrecancion) (CallFunction|SelectNewSong (Variables|Default|GetIndex) :!label _label))
  (Utilities|FlowControl|Sequence
    (:then_0
      (Audio|Components|Audio|SetSound _audiocomponent _selected)
      (Audio|Components|Audio|FadeIn _audiocomponent 0.0 1.0 0.0 "Linear" :!class /Script/Engine.AudioComponent))
    (:then_1
      (Utilities|FlowControl|Delay (Variables|/Script/Engine.SoundBase|GetDuration _selected))
      (goto _label))
    (:then_2
      (bind _asgi_kid_a (Utilities|Casting|CastToGI_KidA (Game|GetGameInstance)))
      (Variables|/Game/Level_Room/Blueprints/Puzzle_Logic/GI_KidA.GI_KidA_C|SetSongName _asgi_kid_a _nombrecancion)
      (bind _asbp_first_person_character (Utilities|Casting|CastToBP_FirstPersonCharacter (Game|GetPlayerCharacter 0)))
      (Default|CallWidget _asbp_first_person_character))))

(fn ConstructionScript)

(fn PlaySong(nofuncioandelay(
  (bind (_audiocomponent _selected _nombrecancion) (CallFunction|SelectNewSong (Variables|Default|GetIndex)))
  (Audio|Components|Audio|SetSound _audiocomponent _selected)
  (Audio|Components|Audio|FadeIn _audiocomponent 1e+01 1.0 0.0 "Linear" :!class /Script/Engine.AudioComponent)
  (Class|SubmixEffectDelayStatics|SetDelayLength (Utilities|Struct|MakeSubmixEffectDelaySettings (Variables|/Script/Engine.SoundBase|GetDuration _selected) 4e+02 (Variables|/Script/Engine.SoundBase|GetDuration _selected)) (Variables|/Script/Engine.SoundBase|GetDuration _selected)))

(fn SelectNewSong
  (params (Index :type Integer))
  (switch int Index
    (:0
      (Variables|Default|SetSongName "Everything in it's right place"))
    (:1
      (Variables|Default|SetSongName "Kid A"))
    (:2
      (Variables|Default|SetSongName "The National Anthem"))
    (:3
      (Variables|Default|SetSongName "How to disappear completely"))
    (:4
      (Variables|Default|SetSongName "Treefingers"))
    (:5
      (Variables|Default|SetSongName "Optimistic"))
    (:6
      (Variables|Default|SetSongName "In limbo"))
    (:7
      (Variables|Default|SetSongName "Idioteque"))
    (:8
      (Variables|Default|SetSongName "Morning bell"))
    (:9
      (Variables|Default|SetSongName "Motion picture soundtrack")))
  (if (<= Index 9)
    (LocalVariables|SetPrevisionalSong (Utilities|Array|Get(acopy) (Variables|Default|GetKidAAlbum) Index))
    (Math|Integer|IncrementInt (Variables|Default|GetIndex)
      (:%20%20
        (return (Variables|Components|GetAudioComponent) (LocalVariables|GetPrevisionalSong) (Variables|Default|GetSongName))))
    (else
      (bind _output_get (Variables|Default|SetIndex 0))
      (CallFunction|SelectNewSong _output_get))))