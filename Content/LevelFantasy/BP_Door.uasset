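; BP_Door is a door actor that slides from its starting location to an Endlocation.
; BeginPlay stores the start location, then Tick accumulates time and lerps the position over Rotationtime, which times translation despite its name.
; Tick disables itself once that time elapses.
; The Opedoors event also disables Tick, so as written it halts movement instead of starting it.
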(event EventOpedoors
  (Actor|Tick|SetActorTickEnabled false))

(event EventTick
  (params (DeltaSeconds :type Float%20%28single-precision%29))
  (Variables|Default|SetcurrentTime (+ DeltaSeconds (Variables|Default|GetcurrentTime)))
  (Transformation|SetActorLocation (Math|Vector|Lerp(Vector) (Variables|Default|GetStartlocation) (Variables|Default|GetEndlocation) (/ (Variables|Default|GetcurrentTime) (Variables|Default|GetRotationtime))) false false)
  (if (>= (Variables|Default|GetcurrentTime) (Variables|Default|GetRotationtime))
    (Actor|Tick|SetActorTickEnabled false)))

(event EventBeginPlay
  (Variables|Default|SetStartlocation (Transformation|GetActorLocation)))

(fn ConstructionScript)