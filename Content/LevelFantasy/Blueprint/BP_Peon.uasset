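; BP_Peon is a rotating-toy puzzle with two giraffes, a horse and a moose that reveals a hidden piece when solved.
; Per-toy triggers open gates that let IA_Interact turn that toy by AngleRotation on a timeline, with input disabled meanwhile.
; BPActivadorJirafa overlaps set flags in Activados, and RecorrerActivados fires PuzzleResuelto when four are true.
; Solving unhides the "Pieza" actor found by display name, plays Win, lowers it and spins it on Tick.
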(event OnComponentBeginOverlap(TriggerActivadorJirafa)
  (params (OverlappedComponent :type Primitive%20Component%20Object%20Reference) (OtherActor :type Actor%20Object%20Reference) (OtherComp :type Primitive%20Component%20Object%20Reference) (OtherBodyIndex :type Integer) (bFromSweep :type Boolean) (SweepResult :type Hit%20Result%20Structure%20%28by%20ref%29))
  (bind _returnvalue (Game|GetPlayerController 0))
  ;[1 1 1 1 80] MOVIMIENTO PERSONAJES
  ;;[1 0.6792 0] JIRAFA
  (Utilities|Casting|CastToBP_FirstPersonCharacter OtherActor)
  (Input|EnableInput (Game|GetPlayerController 0))
  (Utilities|FlowControl|Gate true) ; enters at Open
)

(event OnComponentEndOverlap(TriggerActivadorJirafa)
  (params (OverlappedComponent :type Primitive%20Component%20Object%20Reference) (OtherActor :type Actor%20Object%20Reference) (OtherComp :type Primitive%20Component%20Object%20Reference) (OtherBodyIndex :type Integer))
  (bind _returnvalue (Game|GetPlayerController 0))
  ;[1 1 1 1 80] MOVIMIENTO PERSONAJES
  ;;[1 0.6792 0] JIRAFA
  (Utilities|Casting|CastToBP_FirstPersonCharacter OtherActor)
  (Input|DisableInput (Game|GetPlayerController 0))
  (Utilities|FlowControl|Gate true) ; enters at Close
)

(event OnComponentBeginOverlap(TriggerActivadorPuzzle1)
  (params (OverlappedComponent :type Primitive%20Component%20Object%20Reference) (OtherActor :type Actor%20Object%20Reference) (OtherComp :type Primitive%20Component%20Object%20Reference) (OtherBodyIndex :type Integer) (bFromSweep :type Boolean) (SweepResult :type Hit%20Result%20Structure%20%28by%20ref%29))
  ;[1 1 1 1 80] Setters de completados o no
  ;;[1 0.9307 0.9247] 1 - JIRAFA 2 - CEBRA
  (Utilities|Casting|CastToBPActivadorJirafa OtherActor)
  (Variables|Default|SetJirafa2Activada? true)
  (Utilities|Array|SetArrayElem (Variables|Default|GetActivados) 1 true)
  (CallFunction|RecorrerActivados))

(event OnComponentEndOverlap(TriggerActivadorPuzzle1)
  (params (OverlappedComponent :type Primitive%20Component%20Object%20Reference) (OtherActor :type Actor%20Object%20Reference) (OtherComp :type Primitive%20Component%20Object%20Reference) (OtherBodyIndex :type Integer))
  ;[1 1 1 1 80] Setters de completados o no
  ;;[1 0.9307 0.9247] 1 - JIRAFA 2 - CEBRA
  (Utilities|Casting|CastToBPActivadorJirafa OtherActor)
  (Variables|Default|SetJirafa2Activada? false)
  (Utilities|Array|SetArrayElem (Variables|Default|GetActivados) 1 false))

(event OnComponentBeginOverlap(TriggerActivadorPuzzle2)
  (params (OverlappedComponent :type Primitive%20Component%20Object%20Reference) (OtherActor :type Actor%20Object%20Reference) (OtherComp :type Primitive%20Component%20Object%20Reference) (OtherBodyIndex :type Integer) (bFromSweep :type Boolean) (SweepResult :type Hit%20Result%20Structure%20%28by%20ref%29))
  ;[1 1 1 1 80] Setters de completados o no
  ;;[1 0 0.2456] 2 - CABALLO
  (Utilities|Casting|CastToBPActivadorJirafa OtherActor)
  (Variables|Default|SetCaballoActivada? true)
  (Utilities|Array|SetArrayElem (Variables|Default|GetActivados) 2 true)
  (CallFunction|RecorrerActivados))

(event OnComponentEndOverlap(TriggerActivadorPuzzle2)
  (params (OverlappedComponent :type Primitive%20Component%20Object%20Reference) (OtherActor :type Actor%20Object%20Reference) (OtherComp :type Primitive%20Component%20Object%20Reference) (OtherBodyIndex :type Integer))
  ;[1 1 1 1 80] Setters de completados o no
  ;;[1 0 0.2456] 2 - CABALLO
  (Utilities|Casting|CastToBPActivadorJirafa OtherActor)
  (Variables|Default|SetCaballoActivada? false)
  (Utilities|Array|SetArrayElem (Variables|Default|GetActivados) 2 false))

(event OnComponentBeginOverlap(TriggerActivadorCaballito1)
  (params (OverlappedComponent :type Primitive%20Component%20Object%20Reference) (OtherActor :type Actor%20Object%20Reference) (OtherComp :type Primitive%20Component%20Object%20Reference) (OtherBodyIndex :type Integer) (bFromSweep :type Boolean) (SweepResult :type Hit%20Result%20Structure%20%28by%20ref%29))
  (bind _returnvalue (Game|GetPlayerController 0))
  ;[1 1 1 1 80] MOVIMIENTO PERSONAJES
  ;;[1 0 0.5578] CABALLO
  (Utilities|Casting|CastToBP_FirstPersonCharacter OtherActor)
  (Input|EnableInput (Game|GetPlayerController 0))
  (Utilities|FlowControl|Gate true) ; enters at Open
)

(event OnComponentEndOverlap(TriggerActivadorCaballito1)
  (params (OverlappedComponent :type Primitive%20Component%20Object%20Reference) (OtherActor :type Actor%20Object%20Reference) (OtherComp :type Primitive%20Component%20Object%20Reference) (OtherBodyIndex :type Integer))
  (bind _returnvalue (Game|GetPlayerController 0))
  ;[1 1 1 1 80] MOVIMIENTO PERSONAJES
  ;;[1 0 0.5578] CABALLO
  (Utilities|Casting|CastToBP_FirstPersonCharacter OtherActor)
  (Input|DisableInput (Game|GetPlayerController 0))
  (Utilities|FlowControl|Gate true) ; enters at Close
)

(event OnComponentBeginOverlap(TriggerActivadorPuzzle)
  (params (OverlappedComponent :type Primitive%20Component%20Object%20Reference) (OtherActor :type Actor%20Object%20Reference) (OtherComp :type Primitive%20Component%20Object%20Reference) (OtherBodyIndex :type Integer) (bFromSweep :type Boolean) (SweepResult :type Hit%20Result%20Structure%20%28by%20ref%29))
  ;[1 1 1 1 80] Setters de completados o no
  ;;[1 0.6983 0] 0 - JIRAFA 1
  (Utilities|Casting|CastToBPActivadorJirafa OtherActor)
  (Variables|Default|SetJirafa1Activada? true)
  (Utilities|Array|SetArrayElem (Variables|Default|GetActivados) 0 true)
  (CallFunction|RecorrerActivados))

(event OnComponentBeginOverlap(TriggerActivadorAlce)
  (params (OverlappedComponent :type Primitive%20Component%20Object%20Reference) (OtherActor :type Actor%20Object%20Reference) (OtherComp :type Primitive%20Component%20Object%20Reference) (OtherBodyIndex :type Integer) (bFromSweep :type Boolean) (SweepResult :type Hit%20Result%20Structure%20%28by%20ref%29))
  (bind _returnvalue (Game|GetPlayerController 0))
  ;[1 1 1 1 80] MOVIMIENTO PERSONAJES
  ;;[0 0.117 1] ALCE
  (Utilities|Casting|CastToBP_FirstPersonCharacter OtherActor)
  (Input|EnableInput (Game|GetPlayerController 0))
  (Utilities|FlowControl|Gate true) ; enters at Open
)

(event OnComponentEndOverlap(TriggerActivadorAlce)
  (params (OverlappedComponent :type Primitive%20Component%20Object%20Reference) (OtherActor :type Actor%20Object%20Reference) (OtherComp :type Primitive%20Component%20Object%20Reference) (OtherBodyIndex :type Integer))
  (bind _returnvalue (Game|GetPlayerController 0))
  ;[1 1 1 1 80] MOVIMIENTO PERSONAJES
  ;;[0 0.117 1] ALCE
  (Utilities|Casting|CastToBP_FirstPersonCharacter OtherActor)
  (Input|DisableInput (Game|GetPlayerController 0))
  (Utilities|FlowControl|Gate true) ; enters at Close
)

(event OnComponentBeginOverlap(TriggerActivadorPuzzle3)
  (params (OverlappedComponent :type Primitive%20Component%20Object%20Reference) (OtherActor :type Actor%20Object%20Reference) (OtherComp :type Primitive%20Component%20Object%20Reference) (OtherBodyIndex :type Integer) (bFromSweep :type Boolean) (SweepResult :type Hit%20Result%20Structure%20%28by%20ref%29))
  ;[1 1 1 1 80] Setters de completados o no
  ;;[0 0.1255 1] 3 - ALCE
  (Utilities|Casting|CastToBPActivadorJirafa OtherActor)
  (Variables|Default|SetAlceActivada? true)
  (Utilities|Array|SetArrayElem (Variables|Default|GetActivados) 3 true)
  (CallFunction|RecorrerActivados))

(event OnComponentEndOverlap(TriggerActivadorPuzzle3)
  (params (OverlappedComponent :type Primitive%20Component%20Object%20Reference) (OtherActor :type Actor%20Object%20Reference) (OtherComp :type Primitive%20Component%20Object%20Reference) (OtherBodyIndex :type Integer))
  ;[1 1 1 1 80] Setters de completados o no
  ;;[0 0.1255 1] 3 - ALCE
  (Utilities|Casting|CastToBPActivadorJirafa OtherActor)
  (Variables|Default|SetAlceActivada? false)
  (Utilities|Array|SetArrayElem (Variables|Default|GetActivados) 3 false))

(event OnComponentEndOverlap(TriggerActivadorPuzzle)
  (params (OverlappedComponent :type Primitive%20Component%20Object%20Reference) (OtherActor :type Actor%20Object%20Reference) (OtherComp :type Primitive%20Component%20Object%20Reference) (OtherBodyIndex :type Integer))
  ;[1 1 1 1 80] Setters de completados o no
  ;;[1 0.6983 0] 0 - JIRAFA 1
  (Utilities|Casting|CastToBPActivadorJirafa OtherActor)
  (Variables|Default|SetJirafa1Activada? false)
  (Utilities|Array|SetArrayElem (Variables|Default|GetActivados) 0 false))

(event OnComponentBeginOverlap(TriggerActivadorJirafa1)
  (params (OverlappedComponent :type Primitive%20Component%20Object%20Reference) (OtherActor :type Actor%20Object%20Reference) (OtherComp :type Primitive%20Component%20Object%20Reference) (OtherBodyIndex :type Integer) (bFromSweep :type Boolean) (SweepResult :type Hit%20Result%20Structure%20%28by%20ref%29))
  (bind _returnvalue (Game|GetPlayerController 0))
  ;[1 1 1 1 80] MOVIMIENTO PERSONAJES
  ;;[1 1 1] CEBRA
  (Utilities|Casting|CastToBP_FirstPersonCharacter OtherActor)
  (Input|EnableInput (Game|GetPlayerController 0))
  (Utilities|FlowControl|Gate true) ; enters at Open
)

(event OnComponentEndOverlap(TriggerActivadorJirafa1)
  (params (OverlappedComponent :type Primitive%20Component%20Object%20Reference) (OtherActor :type Actor%20Object%20Reference) (OtherComp :type Primitive%20Component%20Object%20Reference) (OtherBodyIndex :type Integer))
  (bind _returnvalue (Game|GetPlayerController 0))
  ;[1 1 1 1 80] MOVIMIENTO PERSONAJES
  ;;[1 1 1] CEBRA
  (Utilities|Casting|CastToBP_FirstPersonCharacter OtherActor)
  (Input|DisableInput (Game|GetPlayerController 0))
  (Utilities|FlowControl|Gate true) ; enters at Close
)

(event Custom|Puzzle%20Resuelto
  (bind _pieza_local (Variables|Default|GetPieza_Local))
  (Utilities|FlowControl|Sequence
    (:then_0
      (Rendering|SetActorHiddenInGame _pieza_local false)
      (Audio|PlaySound2D "/Game/Level_Room/Sounds/win.win" 1.0 1.0 0.0 0 0)
      (Transformation|AddActorLocalOffset _pieza_local "0.000000,0.000000,-560.000000" false false))
    (:then_1
      (Utilities|FlowControl|Gate true) ; enters at Open
    )))

(event Input|EnhancedActionEvents|EnhancedInputActionIA_Interact
  (params (ActionValue :type Boolean) (ElapsedSeconds :type Float%20%28double-precision%29) (TriggeredSeconds :type Float%20%28double-precision%29) (InputAction :type Input%20Action%20Object%20Reference :default "/Game/FirstPerson/Input/Actions/IA_Interact.IA_Interact"))
  (bind _returnvalue (Game|GetPlayerController 0))
  ;[1 1 1 1 80] MOVIMIENTO PERSONAJES
  ;;[1 0.6792 0] JIRAFA
  (Utilities|FlowControl|Gate true
    (:Exit
      (Input|DisableInput _returnvalue)
      (bind _time (Timeline|TimelineJirafa1 PlayFromStart)
        (:Update
          (Transformation|SetRelativeRotation (Variables|Default|GetS_Toy_Giraffe_ujpheaova_lod3_Var1) (Math|Rotator|Lerp(Rotator) (Variables|Default|GetCurrentRotationJirafa1) (Math|Rotator|MakeRotator (.Roll (Math|Rotator|BreakRotator (Variables|Default|GetCurrentRotationJirafa1))) (.Pitch (Math|Rotator|BreakRotator (Variables|Default|GetCurrentRotationJirafa1))) (+ (.Yaw (Math|Rotator|BreakRotator (Variables|Default|GetCurrentRotationJirafa1))) (Variables|Default|GetAngleRotation))) _time) false false))
        (:Finished
          (Variables|Default|SetCurrentRotationJirafa1 (Math|Rotator|Lerp(Rotator) (Variables|Default|GetCurrentRotationJirafa1) (Math|Rotator|MakeRotator (.Roll (Math|Rotator|BreakRotator (Variables|Default|GetCurrentRotationJirafa1))) (.Pitch (Math|Rotator|BreakRotator (Variables|Default|GetCurrentRotationJirafa1))) (+ (.Yaw (Math|Rotator|BreakRotator (Variables|Default|GetCurrentRotationJirafa1))) (Variables|Default|GetAngleRotation))) _time))
          (Input|EnableInput _returnvalue))))))

(event Input|EnhancedActionEvents|EnhancedInputActionIA_Interact
  (params (ActionValue :type Boolean) (ElapsedSeconds :type Float%20%28double-precision%29) (TriggeredSeconds :type Float%20%28double-precision%29) (InputAction :type Input%20Action%20Object%20Reference :default "/Game/FirstPerson/Input/Actions/IA_Interact.IA_Interact"))
  (bind _returnvalue (Game|GetPlayerController 0))
  ;[1 1 1 1 80] MOVIMIENTO PERSONAJES
  ;;[0 0.117 1] ALCE
  (Utilities|FlowControl|Gate true
    (:Exit
      (Input|DisableInput _returnvalue)
      (bind _time (Timeline|Timeline_1 PlayFromStart)
        (:Update
          (Transformation|SetRelativeRotation (Variables|Default|GetS_Wooden_Toy_Moose_uimjbf0iw_lod3_Var1) (Math|Rotator|Lerp(Rotator) (Variables|Default|GetCurrentRotationAlce) (Math|Rotator|MakeRotator (.Roll (Math|Rotator|BreakRotator (Variables|Default|GetCurrentRotationAlce))) (.Pitch (Math|Rotator|BreakRotator (Variables|Default|GetCurrentRotationAlce))) (+ (.Yaw (Math|Rotator|BreakRotator (Variables|Default|GetCurrentRotationAlce))) (Variables|Default|GetAngleRotation))) _time) false false))
        (:Finished
          (Variables|Default|SetCurrentRotationAlce (Math|Rotator|Lerp(Rotator) (Variables|Default|GetCurrentRotationAlce) (Math|Rotator|MakeRotator (.Roll (Math|Rotator|BreakRotator (Variables|Default|GetCurrentRotationAlce))) (.Pitch (Math|Rotator|BreakRotator (Variables|Default|GetCurrentRotationAlce))) (+ (.Yaw (Math|Rotator|BreakRotator (Variables|Default|GetCurrentRotationAlce))) (Variables|Default|GetAngleRotation))) _time))
          (Input|EnableInput _returnvalue))))))

(event Input|EnhancedActionEvents|EnhancedInputActionIA_Interact
  (params (ActionValue :type Boolean) (ElapsedSeconds :type Float%20%28double-precision%29) (TriggeredSeconds :type Float%20%28double-precision%29) (InputAction :type Input%20Action%20Object%20Reference :default "/Game/FirstPerson/Input/Actions/IA_Interact.IA_Interact"))
  (bind _returnvalue (Game|GetPlayerController 0))
  ;[1 1 1 1 80] MOVIMIENTO PERSONAJES
  ;;[1 0 0.5578] CABALLO
  (Utilities|FlowControl|Gate true
    (:Exit
      (Input|DisableInput _returnvalue)
      (bind _time (Timeline|Timeline_0 PlayFromStart)
        (:Update
          (Transformation|SetRelativeRotation (Variables|Default|GetS_Wooden_Toy_Horse_uhcjdhpva_lod3_Var1) (Math|Rotator|Lerp(Rotator) (Variables|Default|GetCurrentRotationCaballo) (Math|Rotator|MakeRotator (.Roll (Math|Rotator|BreakRotator (Variables|Default|GetCurrentRotationCaballo))) (.Pitch (Math|Rotator|BreakRotator (Variables|Default|GetCurrentRotationCaballo))) (+ (.Yaw (Math|Rotator|BreakRotator (Variables|Default|GetCurrentRotationCaballo))) (Variables|Default|GetAngleRotation))) _time) false false))
        (:Finished
          (Variables|Default|SetCurrentRotationCaballo (Math|Rotator|Lerp(Rotator) (Variables|Default|GetCurrentRotationCaballo) (Math|Rotator|MakeRotator (.Roll (Math|Rotator|BreakRotator (Variables|Default|GetCurrentRotationCaballo))) (.Pitch (Math|Rotator|BreakRotator (Variables|Default|GetCurrentRotationCaballo))) (+ (.Yaw (Math|Rotator|BreakRotator (Variables|Default|GetCurrentRotationCaballo))) (Variables|Default|GetAngleRotation))) _time))
          (Input|EnableInput _returnvalue))))))

(event Input|EnhancedActionEvents|EnhancedInputActionIA_Interact
  (params (ActionValue :type Boolean) (ElapsedSeconds :type Float%20%28double-precision%29) (TriggeredSeconds :type Float%20%28double-precision%29) (InputAction :type Input%20Action%20Object%20Reference :default "/Game/FirstPerson/Input/Actions/IA_Interact.IA_Interact"))
  (bind _returnvalue (Game|GetPlayerController 0))
  ;[1 1 1 1 80] MOVIMIENTO PERSONAJES
  ;;[1 1 1] CEBRA
  (Utilities|FlowControl|Gate true
    (:Exit
      (Input|DisableInput _returnvalue)
      (bind _time (Timeline|Timeline PlayFromStart)
        (:Update
          (Transformation|SetRelativeRotation (Variables|Default|GetS_Toy_Giraffe_ujpheaova_lod3_Var2) (Math|Rotator|Lerp(Rotator) (Variables|Default|GetCurrentRotationJirafa2) (Math|Rotator|MakeRotator (.Roll (Math|Rotator|BreakRotator (Variables|Default|GetCurrentRotationJirafa2))) (.Pitch (Math|Rotator|BreakRotator (Variables|Default|GetCurrentRotationJirafa2))) (+ (.Yaw (Math|Rotator|BreakRotator (Variables|Default|GetCurrentRotationJirafa2))) (Variables|Default|GetAngleRotation))) _time) false false))
        (:Finished
          (Variables|Default|SetCurrentRotationJirafa2 (Math|Rotator|Lerp(Rotator) (Variables|Default|GetCurrentRotationJirafa2) (Math|Rotator|MakeRotator (.Roll (Math|Rotator|BreakRotator (Variables|Default|GetCurrentRotationJirafa2))) (.Pitch (Math|Rotator|BreakRotator (Variables|Default|GetCurrentRotationJirafa2))) (+ (.Yaw (Math|Rotator|BreakRotator (Variables|Default|GetCurrentRotationJirafa2))) (Variables|Default|GetAngleRotation))) _time))
          (Input|EnableInput _returnvalue))))))

(event EventTick
  (params (DeltaSeconds :type Float%20%28single-precision%29))
  (Utilities|FlowControl|Gate true
    (:Exit
      (Transformation|AddActorLocalRotation (Variables|Default|GetPieza_Local) (Math|Rotator|MakeRotator 0.0 0.0 (* DeltaSeconds (Variables|Default|GetRotation))) false false))))

(event EventBeginPlay
  (Utilities|FlowControl|Sequence
    (:then_0
      (Variables|Default|SetCurrentRotationJirafa1 (Transformation|GetWorldRotation (Variables|Default|GetS_Toy_Giraffe_ujpheaova_lod3_Var1)))
      (Variables|Default|SetCurrentRotationJirafa2 (Transformation|GetWorldRotation (Variables|Default|GetS_Toy_Giraffe_ujpheaova_lod3_Var2)))
      (Variables|Default|SetCurrentRotationCaballo (Transformation|GetWorldRotation (Variables|Default|GetS_Wooden_Toy_Horse_uhcjdhpva_lod3_Var1)))
      (Variables|Default|SetCurrentRotationAlce (Transformation|GetWorldRotation (Variables|Default|GetS_Wooden_Toy_Moose_uimjbf0iw_lod3_Var1))))
    (:then_1
      ;[1 1 1] escondemos el puzzle
      (bind _outactors (Actor|GetAllActorsOfClass "/Script/Engine.Actor"))
      (bind _array_element (Utilities|Array|ForEachLoopwithBreak _outactors :!label _label)
        (:LoopBody
          (if (Utilities|Enum|Equal(Enum) (Utilities|GetDisplayName _array_element) "Pieza")
            (bind _output_get (Variables|Default|SetPieza_Local _array_element))
            (Rendering|SetActorHiddenInGame _output_get true)
            (goto _label Break)))))))

(fn ConstructionScript)

(fn RecorrerActivados
  (Variables|Default|SetActivadosCant 0)
  (bind _array_element (Utilities|Array|ForEachLoopwithBreak (Variables|Default|GetActivados) :!label _label)
    (:LoopBody
      (if _array_element
        (Math|Integer|IncrementInt (Variables|Default|GetActivadosCant))
        (else
          (goto _label Break))))
    (:Completed
      (if (== (Variables|Default|GetActivadosCant) 4)
        (CallFunction|PuzzleResuelto)))))