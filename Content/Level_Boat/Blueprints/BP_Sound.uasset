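; BP_Sound is a one-shot sound trigger in the boat level, fired when the first-person character enters its Box.
; The begin overlap passes a DoOnce, calls FadeIn on Audio, then FadeOut immediately with no delay between, and destroys the actor after a short delay.
; Debug strings print on overlap and playback; end overlap only casts and does nothing further.
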(event OnComponentBeginOverlap(Box)
  (params (OverlappedComponent :type Primitive%20Component%20Object%20Reference) (OtherActor :type Actor%20Object%20Reference) (OtherComp :type Primitive%20Component%20Object%20Reference) (OtherBodyIndex :type Integer) (bFromSweep :type Boolean) (SweepResult :type Hit%20Result%20Structure%20%28by%20ref%29))
  (Development|PrintString "en el trigger")
  (Utilities|Casting|CastToBP_FirstPersonCharacter OtherActor)
  (Utilities|FlowControl|DoOnce false
    (:Completed
      (Audio|Components|Audio|FadeIn (Variables|Default|GetAudio) 1.0 1.0 0.0 "Linear" :!class /Script/Engine.AudioComponent)
      (Development|PrintString "reproduciendo")
      (Audio|Components|Audio|FadeOut (Variables|Default|GetAudio) 1.0 0.0 "Linear" :!class /Script/Engine.AudioComponent)
      (Utilities|FlowControl|Delay 2.6)
      (Actor|DestroyActor))))

(event OnComponentEndOverlap(Box)
  (params (OverlappedComponent :type Primitive%20Component%20Object%20Reference) (OtherActor :type Actor%20Object%20Reference) (OtherComp :type Primitive%20Component%20Object%20Reference) (OtherBodyIndex :type Integer))
  (Utilities|Casting|CastToBP_FirstPersonCharacter OtherActor))

(event EventBeginPlay)

(event Collision|EventActorBeginOverlap
  (params (OtherActor :type Actor%20Object%20Reference)))

(event EventTick
  (params (DeltaSeconds :type Float%20%28single-precision%29)))

(fn ConstructionScript)