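; UDS component that measures how enclosed the player's surroundings are, producing an occlusion profile.
; A looping timer fires line traces upward and around the camera or stored location, deriving directional, blended directional, overall and optional rain-direction openness values.
; Being below water level or forcing full occlusion zeroes the profile.
; Tick eases the current profile toward that target at per-channel speeds and updates the inverted global occlusion.
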(event EventTick
  (params (DeltaSeconds :type Float%20%28single-precision%29))
  (CallFunction|UpdateCurrentOcclusionProfile))

(fn UpdateTargetOcclusionProfile
  (bind _returnvalue (Game|Player|GetPlayerPawn 0))
  (CallFunction|GetOcclusionLocation)
  (Utilities|IsValid _returnvalue
    (:Is%20Valid
      (Utilities|Array|Add (LocalVariables|GetActors%20to%20Ignore) _returnvalue))
    (:Is%20Not%20Valid
      _))
  (if (or (and (< (.Z (Math|Vector|BreakVector (Variables|Default|GetOcclusion%20Location))) (Variables|Default|GetWater%20Level)) (Variables|Default|GetUse%20Water%20Level)) (Variables|Default|GetForce%20Full%20Occlusion))
    (Variables|Default|SetTarget%20Occlusion%20Profile (Utilities|Array|MakeArray 0.0 0.0 0.0 0.0 0.0 0.0 0.0 0.0 0.0 0.0))
    (else
      (for _index (range 0 4)
        (bind _returnvalue_2 (Collision|LineTraceByChannel (Variables|Default|GetOcclusion%20Location) (+ (* (Math|Vector|Normalize (+ (* (Utilities|Array|Get(acopy) (Utilities|Array|MakeArray "0, 0, 0" "1.000000, 0, 0" "0,1.000000, 0" "-1.000000, 0, 0" "0,-1.000000, 0") _index) 0.35) "0, 0,1.000000")) (Variables|Default|GetMax%20Interior%20Occlusion%20Distance)) (Variables|Default|GetOcclusion%20Location)) (Variables|Default|GetOcclusion%20Trace%20Channel) false (LocalVariables|GetActors%20to%20Ignore) "None" true "(R=1.000000,G=0.000000,B=0.000000,A=1.000000)" "(R=0.000000,G=1.000000,B=0.000000,A=1.000000)" 0.5))
        (if _returnvalue_2
          (Math|Integer|IncrementInt (LocalVariables|GetTotal%20Hits))))
      (for _array_element (Utilities|Array|MakeArray "1.000000, 0, 0" "0,1.000000, 0" "-1.000000, 0, 0" "0,-1.000000, 0")
        (LocalVariables|SetDirectional%20Hits 0)
        (for _index_2 (range -1 1)
          (for _index_3 (range 0 1)
            (bind _returnvalue_3 (Collision|LineTraceByChannel (Variables|Default|GetOcclusion%20Location) (+ (* (Math|Vector|Normalize (+ (Math|Vector|RotateVectorAroundAxis _array_element (* _index_2 3e+01) "0, 0,1.000000") (Math|Vector|MakeVector 0.0 0.0 (+ (* _index_3 0.35) 0.1)))) (Variables|Default|GetMax%20Interior%20Occlusion%20Distance)) (Variables|Default|GetOcclusion%20Location)) (Variables|Default|GetOcclusion%20Trace%20Channel) false (LocalVariables|GetActors%20to%20Ignore) "None" true "(R=1.000000,G=0.000000,B=0.000000,A=1.000000)" "(R=0.000000,G=1.000000,B=0.000000,A=1.000000)" 0.5))
            (if _returnvalue_3
              (Math|Integer|IncrementInt (LocalVariables|GetTotal%20Hits)
                (:%20%20
                  (Math|Integer|IncrementInt (LocalVariables|GetDirectional%20Hits)))))))
        (Utilities|Array|Add (LocalVariables|GetNew%20Occlusion%20Profile) (Math|Float|MapRangeClamped (Math|Conversions|ToFloat(Integer) (LocalVariables|GetDirectional%20Hits)) 0.0 6.0 1.0 0.0)))
      (LocalVariables|SetTotal%20Occlusion (Math|Float|MapRangeClamped (Math|Conversions|ToFloat(Integer) (LocalVariables|GetTotal%20Hits)) (* (Variables|Default|GetNot%20Occluded%20Percent) 29.0) (* (Variables|Default|GetFull%20Occluded%20Percent) 29.0) 1.0 0.0))
      (for _index_4 (range 0 3)
        (Utilities|Array|Add (LocalVariables|GetNew%20Occlusion%20Profile) (* (Math|Float|Lerp (Utilities|Array|Get(acopy) (LocalVariables|GetNew%20Occlusion%20Profile) _index_4) (LocalVariables|GetTotal%20Occlusion) 0.25) (Math|Float|MapRangeClamped (LocalVariables|GetTotal%20Occlusion) 0.0 0.2 0.0 1.0))))
      (Utilities|Array|Add (LocalVariables|GetNew%20Occlusion%20Profile) (LocalVariables|GetTotal%20Occlusion))
      (if (Variables|Default|GetCalculate%20Rain%20Occlusion)
        (bind _returnvalue_4 (Collision|LineTraceByChannel (Variables|Default|GetOcclusion%20Location) (+ (Variables|Default|GetOcclusion%20Location) (* (Math|Vector|Normalize (* (Variables|Default|GetRain%20Velocity) -1.0)) (Variables|Default|GetMax%20Interior%20Occlusion%20Distance))) (Variables|Default|GetOcclusion%20Trace%20Channel) false (LocalVariables|GetActors%20to%20Ignore) "None" true "(R=1.000000,G=0.000000,B=0.000000,A=1.000000)" "(R=0.000000,G=1.000000,B=0.000000,A=1.000000)" 0.5))
        (Utilities|Array|Add (LocalVariables|GetNew%20Occlusion%20Profile) (Math|Float|Lerp (Math|Float|SelectFloat 0.0 1.0 _returnvalue_4) (* (Math|Float|SelectFloat 0.0 1.0 _returnvalue_4) (LocalVariables|GetTotal%20Occlusion)) 0.5))
        (Variables|Default|SetTarget%20Occlusion%20Profile (LocalVariables|GetNew%20Occlusion%20Profile))
        (else
          (Utilities|Array|Add (LocalVariables|GetNew%20Occlusion%20Profile) 0.0)
          (Variables|Default|SetTarget%20Occlusion%20Profile (LocalVariables|GetNew%20Occlusion%20Profile)))))))

(fn UpdateCurrentOcclusionProfile
  (LocalVariables|SetInterp%20Speed%20Multiplier (/ 1.0 (Variables|Default|GetOcclusion%20Update%20Period)))
  (for (_array_element _array_index) (Variables|Default|GetCurrent%20Occlusion%20Profile)
    (Utilities|Array|SetArrayElem (Variables|Default|GetCurrent%20Occlusion%20Profile) _array_index (Math|Interpolation|FInterpTo _array_element (Utilities|Array|Get(acopy) (Variables|Default|GetTarget%20Occlusion%20Profile) _array_index) (Utilities|Time|GetWorldDeltaSeconds) (* (Math|Float|SelectFloat 5.0 (Math|Float|SelectFloat 1.4 0.6 (< _array_index 4)) (== _array_index 9)) (LocalVariables|GetInterp%20Speed%20Multiplier)))))
  (Variables|Default|SetInverted%20Global%20Occlusion (- 1.0 (Utilities|Array|Get(acopy) (Variables|Default|GetCurrent%20Occlusion%20Profile) 8))))

(fn Initialize
  (Components|Tick|SetComponentTickEnabled true)
  (CallFunction|UpdateTargetOcclusionProfile)
  (Variables|Default|SetCurrent%20Occlusion%20Profile (Variables|Default|GetTarget%20Occlusion%20Profile))
  (Class|KismetSystemLibrary|SetTimerforNextTick 0 "Get Starting Occlusion Profile"))

(fn GetStartingOcclusionProfile
  (CallFunction|GetOcclusionLocation)
  (if (Utilities|Operators|EqualEqual :A (Variables|Default|GetOcclusion%20Location))
    (Class|KismetSystemLibrary|SetTimerforNextTick 0 "Get Starting Occlusion Profile")
    (else
      (CallFunction|UpdateTargetOcclusionProfile)
      (Variables|Default|SetCurrent%20Occlusion%20Profile (Variables|Default|GetTarget%20Occlusion%20Profile))
      (Utilities|Time|SetTimerbyFunctionName 0 "Update Target Occlusion Profile" (Variables|Default|GetOcclusion%20Update%20Period) true)
      (Variables|Default|SetRunning true))))

(fn GetOcclusionLocation
  (bind _returnvalue (Game|GetPlayerCameraManager 0))
  (if (Variables|Default|GetAcquire%20Camera%20Location)
    (Utilities|IsValid _returnvalue
      (:Is%20Valid
        (Variables|Default|SetOcclusion%20Location (Camera|GetCameraLocation _returnvalue))))))