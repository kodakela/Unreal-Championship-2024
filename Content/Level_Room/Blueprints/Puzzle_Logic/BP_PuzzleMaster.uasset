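; BP_PuzzleMaster holds the shared state of an item-placement puzzle: a Data array of puzzle entries and a GameCompleted flag.
; GiveItemToPuzzle marks the indexed entry as placed, fires the empty PlaceItem event, then recomputes GameCompleted.
; That check clears its all-done flag at the first entry whose ItemPlaced is true, which looks inverted for a completion test.
; ReturnPuzzleData exposes the array to callers.
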(event Custom|Place%20Item
  (params (Index :type Integer) (Item :type Data%20Table%20Row%20Handle%20Structure)))

(fn ConstructionScript)

(fn GiveItemtoPuzzle
  (params (Item :type Data%20Table%20Row%20Handle%20Structure) (Index :type Integer))
  (bind _structout (Utilities|Struct|SetmembersinS_PuzzleData (Utilities|Array|Get(acopy) (Variables|Default|GetData) Index) true))
  (Utilities|Array|SetArrayElem (Variables|Default|GetData) Index _structout)
  (CallFunction|PlaceItem Index Item)
  (bind _array_element (Utilities|Array|ForEachLoopwithBreak (Variables|Default|GetData) :!label _label)
    (:LoopBody
      (if (Utilities|Struct|BreakS_PuzzleData _array_element)
        (LocalVariables|SetL_AllDone false)
        (goto _label Break)))
    (:Completed
      (Variables|Default|SetGame_Completed (LocalVariables|GetL_AllDone)))))

(fn ReturnPuzzleData
  (return (Variables|Default|GetData)))