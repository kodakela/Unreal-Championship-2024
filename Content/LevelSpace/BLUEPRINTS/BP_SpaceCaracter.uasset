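; Player-controlled spaceship character for the space level, with look, thrust and sideways movement.
; BeginPlay adds the ship's Enhanced Input mapping context, and the look action feeds controller yaw and pitch.
; Input events set flags that Tick turns into movement along actor forward or the world Y axis, adding or subtracting rates with DeltaSeconds.
; The brake flag (Frenar) is never read, and releasing left (Izq) leaves its flag true.
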(event Input|EnhancedActionEvents|EnhancedInputActionIA_LookShip
  (params (ActionValue :type Vector%202D%20Structure) (ElapsedSeconds :type Float%20%28double-precision%29) (TriggeredSeconds :type Float%20%28double-precision%29) (InputAction :type Input%20Action%20Object%20Reference :default "/Game/LevelSpace/INPUT/IA_LookShip.IA_LookShip"))
  (Pawn|Input|AddControllerYawInput (.x ActionValue))
  (Pawn|Input|AddControllerPitchInput (.y ActionValue)))

(event EventBeginPlay
  ;[0 0 0] Imput Mapping Call
  (bind _asplayer_controller (Utilities|Casting|CastToPlayerController (Pawn|GetController)))
  (Utilities|IsValid (PlayerController|LocalPlayerSubsystems|GetEnhancedInputLocalPlayerSubsystem _asplayer_controller)
    (:Is%20Valid
      (Input|AddMappingContext (PlayerController|LocalPlayerSubsystems|GetEnhancedInputLocalPlayerSubsystem _asplayer_controller) "/Game/LevelSpace/INPUT/IM_ImputMappingShip.IM_ImputMappingShip" 0 "(bIgnoreAllPressedKeysUntilRelease=True,bForceImmediately=False,bNotifyUserSettings=False)"))))

(event Collision|EventActorBeginOverlap
  (params (OtherActor :type Actor%20Object%20Reference)))

(event EventTick
  (params (DeltaSeconds :type Float%20%28single-precision%29))
  (Utilities|FlowControl|Sequence
    (:then_0
      (if (Variables|Default|GetAcelerar)
        (Pawn|Input|AddMovementInput (Transformation|GetActorForwardVector) (+ DeltaSeconds (Variables|Default|GetTasa%20de%20Aceleración)) false)))
    (:then_1
      (if (Variables|Default|GetDerecha)
        (Pawn|Input|AddMovementInput (Math|Vector|GetRightVector "0, 0, 0") (+ DeltaSeconds (Variables|Default|GetTasa%20de%20Giro)) false)))
    (:then_2
      (if (Variables|Default|GetIzq)
        (Pawn|Input|AddMovementInput (Math|Vector|GetRightVector "0, 0, 0") (- DeltaSeconds (Variables|Default|GetTasa%20de%20Giro)) false)))))

(event Input|ActionEvents|InputActionAcelerar
  (params (Key :type Key%20Structure :default "None"))
  (:Pressed
    (Variables|Default|SetAcelerar true))
  (:Released
    (Variables|Default|SetAcelerar false)))

(event Input|ActionEvents|InputActionDerecha
  (params (Key :type Key%20Structure :default "None"))
  (:Pressed
    (Variables|Default|SetDerecha true))
  (:Released
    (Variables|Default|SetDerecha false)))

(event Input|ActionEvents|InputActionIzq
  (params (Key :type Key%20Structure :default "None"))
  (:Pressed
    (Variables|Default|SetIzq true))
  (:Released
    (Variables|Default|SetIzq true)))

(event Input|ActionEvents|InputActionFrenar
  (params (Key :type Key%20Structure :default "None"))
  (:Pressed
    (Variables|Default|SetFrenar true))
  (:Released
    (Variables|Default|SetFrenar false)))

(fn ConstructionScript)