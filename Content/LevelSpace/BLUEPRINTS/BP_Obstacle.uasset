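; BP_Obstacle is a drifting, tumbling asteroid obstacle for the space level.
; On BeginPlay it gives its RotatingMovement component a random rotation rate on each axis within a shared min/max range.
; After a short delay it launches the Asteroids component with a random X-axis impulse scaled by Force, applied as a velocity change so mass is ignored.
; Overlap, Tick and the construction script are empty.
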(event EventBeginPlay
  (bind _minrotation (Variables|Default|GetminRotation))
  (bind _maxrotation (Variables|Default|GetmaxRotation))
  (bind _returnvalue (Math|Random|RandomFloatinRange _minrotation _maxrotation))
  (Variables|/Script/Engine.RotatingMovementComponent|SetRotationRate (Variables|Default|GetRotatingMovement) (Math|Rotator|MakeRotator _returnvalue _returnvalue _returnvalue))
  (Utilities|FlowControl|Delay 3.0)
  (Physics|AddImpulse (Variables|Default|GetAsteroids) (* (Math|Vector|MakeVector (Math|Random|RandomFloatinRange (Variables|Default|GetminiImpulse) (Variables|Default|GetmaxImpulse)) 0.0 0.0) (Variables|Default|GetForce)) "None" true))

(event Collision|EventActorBeginOverlap
  (params (OtherActor :type Actor%20Object%20Reference)))

(event EventTick
  (params (DeltaSeconds :type Float%20%28single-precision%29)))

(fn ConstructionScript)