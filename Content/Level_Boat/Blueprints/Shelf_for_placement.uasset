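; Colour-matching placement shelf in the boat level that accepts snowballs and triggers a door.
; When a BP_Snowball overlaps the shelf, its colour is compared to the shelf's colour within a small tolerance.
; A match sets Correct, stops the snowball's physics and calls OpenDoor on the IsCorrect_Door actor found by class lookup.
; A mismatch only clears Correct.
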(event OnComponentBeginOverlap(Shelf)
  (params (OverlappedComponent :type Primitive%20Component%20Object%20Reference) (OtherActor :type Actor%20Object%20Reference) (OtherComp :type Primitive%20Component%20Object%20Reference) (OtherBodyIndex :type Integer) (bFromSweep :type Boolean) (SweepResult :type Hit%20Result%20Structure%20%28by%20ref%29))
  (if (Utilities|ClassIsChildOf (Utilities|GetClass OtherActor) "/Game/Level_Boat/Blueprints/BP_Snowball.BP_Snowball_C")
    (bind _asbp_snowball (Utilities|Casting|CastToBP_Snowball OtherActor))
    (if (Class|KismetMathLibrary|LinearColorIsNearEqual (Math|Conversions|ToLinearColor(Color) (Variables|/Game/Level_Boat/Blueprints/BP_Snowball.BP_Snowball_C|GetColor _asbp_snowball)) (Math|Conversions|ToLinearColor(Color) (Variables|Default|GetColor%20)) 0.1)
      (Variables|Default|SetCorrect true)
      (Physics|SetSimulatePhysics (Variables|/Game/Level_Boat/Blueprints/BP_Snowball.BP_Snowball_C|GetSnowball _asbp_snowball) false)
      ;[1 0.8142 0.003424] no llamé a isCorrectDoor
      (bind _returnvalue (Actor|GetActorOfClass "/Game/Level_Boat/Blueprints/IsCorrect_Door.IsCorrect_Door_C"))
      (Default|OpenDoor _returnvalue)
      (else
        (Variables|Default|SetCorrect false)))))

(fn ConstructionScript)