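; Hint trigger volume that lets the player press E inside its box to show or hide TextRenderActor hints for the current level.
; BeginPlay hides all TextRenderActors, and box overlaps open and close a gate on the E key.
; GI_KidA's ActualLevel selects one of three hint pairs; successive presses show then hide one hint before switching to the other, with a pickup sound.
; Hints are addressed by hard-coded GetAllActorsOfClass indices, tracked in HintIsHidden.
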(event OnComponentEndOverlap(Box)
  (params (OverlappedComponent :type Primitive%20Component%20Object%20Reference) (OtherActor :type Actor%20Object%20Reference) (OtherComp :type Primitive%20Component%20Object%20Reference) (OtherBodyIndex :type Integer))
  (bind _hintishidden (Variables|Default|GetHintIsHidden))
  (bind _hintishidden_2 (Variables|Default|GetHintIsHidden))
  (bind _hintishidden_3 (Variables|Default|GetHintIsHidden))
  (Input|EnableInput (Game|GetPlayerController 0))
  (Utilities|FlowControl|Gate true) ; enters at Close
)

(event OnComponentBeginOverlap(Box)
  (params (OverlappedComponent :type Primitive%20Component%20Object%20Reference) (OtherActor :type Actor%20Object%20Reference) (OtherComp :type Primitive%20Component%20Object%20Reference) (OtherBodyIndex :type Integer) (bFromSweep :type Boolean) (SweepResult :type Hit%20Result%20Structure%20%28by%20ref%29))
  (bind _hintishidden (Variables|Default|GetHintIsHidden))
  (bind _hintishidden_2 (Variables|Default|GetHintIsHidden))
  (bind _hintishidden_3 (Variables|Default|GetHintIsHidden))
  (Input|EnableInput (Game|GetPlayerController 0))
  (Utilities|FlowControl|Gate true) ; enters at Open
)

(event Input|EnhancedActionEvents|EnhancedInputActionIA_Interact
  (params (ActionValue :type Boolean) (ElapsedSeconds :type Float%20%28double-precision%29) (TriggeredSeconds :type Float%20%28double-precision%29) (InputAction :type Input%20Action%20Object%20Reference :default "/Game/FirstPerson/Input/Actions/IA_Interact.IA_Interact")))

(event EventBeginPlay
  (bind _outactors (Actor|GetAllActorsOfClass "/Script/Engine.TextRenderActor"))
  (for _array_element _outactors
    (Rendering|SetActorHiddenInGame _array_element true)))

(event Input|KeyboardEvents|E
  (params (Key :type Key%20Structure :default "None"))
  (bind _hintishidden (Variables|Default|GetHintIsHidden))
  (bind _hintishidden_2 (Variables|Default|GetHintIsHidden))
  (bind _hintishidden_3 (Variables|Default|GetHintIsHidden))
  (:Pressed
    (Utilities|FlowControl|Gate true
      (:Exit
        (bind _asgi_kid_a (Utilities|Casting|CastToGI_KidA (Game|GetGameInstance)))
        (switch int (Variables|/Game/Level_Room/Blueprints/Puzzle_Logic/GI_KidA.GI_KidA_C|GetActualLevel _asgi_kid_a)
          (:0
            ;[1 1 1] p modularizar
            (if (Variables|Default|GetL1)
              (bind _outactors (Actor|GetAllActorsOfClass "/Script/Engine.TextRenderActor"))
              (if (Utilities|Array|Get(acopy) _hintishidden_3)
                (Rendering|SetActorHiddenInGame (Utilities|Array|Get(acopy) _outactors) false)
                (Utilities|Array|SetArrayElem _hintishidden_3 0 false)
                (else
                  (Rendering|SetActorHiddenInGame (Utilities|Array|Get(acopy) _outactors) true)
                  (Utilities|Array|SetArrayElem _hintishidden_3 0 true)
                  (Variables|Default|SetL1 false)))
              (else
                (bind _outactors_2 (Actor|GetAllActorsOfClass "/Script/Engine.TextRenderActor"))
                (if (Utilities|Array|Get(acopy) _hintishidden_3 1)
                  (Rendering|SetActorHiddenInGame (Utilities|Array|Get(acopy) _outactors_2 1) false)
                  (Utilities|Array|SetArrayElem _hintishidden_3 1 false)
                  (else
                    (Rendering|SetActorHiddenInGame (Utilities|Array|Get(acopy) _outactors_2 1) true)
                    (Utilities|Array|SetArrayElem _hintishidden_3 1 true)
                    (Variables|Default|SetL1 true))))))
          (:1
            (if (Variables|Default|GetL2)
              (bind _outactors_3 (Actor|GetAllActorsOfClass "/Script/Engine.TextRenderActor"))
              (if (Utilities|Array|Get(acopy) _hintishidden_2 2)
                (Rendering|SetActorHiddenInGame (Utilities|Array|Get(acopy) _outactors_3 2) false)
                (Utilities|Array|SetArrayElem _hintishidden_2 2 false)
                (else
                  (Rendering|SetActorHiddenInGame (Utilities|Array|Get(acopy) _outactors_3 2) true)
                  (Utilities|Array|SetArrayElem _hintishidden_2 2 true)
                  (Variables|Default|SetL2 false)))
              (else
                (bind _outactors_4 (Actor|GetAllActorsOfClass "/Script/Engine.TextRenderActor"))
                (if (Utilities|Array|Get(acopy) _hintishidden_2 3)
                  (Rendering|SetActorHiddenInGame (Utilities|Array|Get(acopy) _outactors_4 3) false)
                  (Utilities|Array|SetArrayElem _hintishidden_2 3 false)
                  (else
                    (Rendering|SetActorHiddenInGame (Utilities|Array|Get(acopy) _outactors_4 3) true)
                    (Utilities|Array|SetArrayElem _hintishidden_2 3 true)
                    (Variables|Default|SetL2 true))))))
          (:2
            (if (Variables|Default|GetL3)
              (bind _outactors_5 (Actor|GetAllActorsOfClass "/Script/Engine.TextRenderActor"))
              (if (Utilities|Array|Get(acopy) _hintishidden 4)
                (Rendering|SetActorHiddenInGame (Utilities|Array|Get(acopy) _outactors_5 4) false)
                (Utilities|Array|SetArrayElem _hintishidden 4 false)
                (else
                  (Rendering|SetActorHiddenInGame (Utilities|Array|Get(acopy) _outactors_5 4) true)
                  (Utilities|Array|SetArrayElem _hintishidden 4 true)
                  (Variables|Default|SetL3 false)))
              (else
                (bind _outactors_6 (Actor|GetAllActorsOfClass "/Script/Engine.TextRenderActor"))
                (if (Utilities|Array|Get(acopy) _hintishidden 5)
                  (Rendering|SetActorHiddenInGame (Utilities|Array|Get(acopy) _outactors_6 5) false)
                  (Utilities|Array|SetArrayElem _hintishidden 5 false)
                  (else
                    (Rendering|SetActorHiddenInGame (Utilities|Array|Get(acopy) _outactors_6 5) true)
                    (Utilities|Array|SetArrayElem _hintishidden 5 true)
                    (Variables|Default|SetL3 true)))))))
        (Audio|PlaySound2D "/Game/Level_Room/Sounds/pick_up.pick_up" 1.0 1.0 0.0 0 0)))))

(fn ConstructionScript)

(fn ShowText
  (params (Actor :type Actor%20Object%20Reference)))

(fn HideActor
  (params (Actor :type Actor%20Object%20Reference))
  (Rendering|SetActorHiddenInGame Actor true))