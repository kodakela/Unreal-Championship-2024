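; Player component that lets its owning actor place inventory items into puzzle actors in front of it.
; InteractWithPuzzle box-traces forward on the Camera channel with debug drawing, then fetches puzzle data and inventory through message calls.
; It matches inventory row names against unfilled slots and passes a match to the puzzle, breaking out of the loops.
; The inventory removal call is disconnected, so items stay with the owner.
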(event EventBeginPlay)

(event EventTick
  (params (DeltaSeconds :type Float%20%28single-precision%29)))

(fn InteractwithPuzzle
  (bind _returnvalue (Components|GetOwner))
  (bind _returnvalue_2 (Transformation|GetActorLocation _returnvalue))
  (bind (_outhit _returnvalue_3) (Collision|BoxTraceByChannel _returnvalue_2 (+ _returnvalue_2 (* (Transformation|GetActorForwardVector _returnvalue) 1000)) "20.000000,20.000000,20.000000" "0, 0, 0" "TraceTypeQuery2" false 0 "ForDuration"))
  (if _returnvalue_3
    (bind _output_get (LocalVariables|SetL_HitActor (.HitActor (Collision|BreakHitResult _outhit))))
    (bind _data (Class|PuzzleInterface|ReturnPuzzleData(Message) _output_get))
    (LocalVariables|SetL_PuzzleData _data)
    (bind _items (Class|InventoryInterface|ReturnInventory(Message) (Components|GetOwner)))
    (LocalVariables|SetL_Inventory _items)
    (bind (_array_element _array_index) (Utilities|Array|ForEachLoopwithBreak (LocalVariables|GetL_PuzzleData) :!label _label)
      (:LoopBody
        (if (not (.ItemPlaced (Utilities|Struct|BreakS_PuzzleData _array_element)))
          (bind (_array_element_2 _array_index_2) (Utilities|Array|ForEachLoopwithBreak (LocalVariables|GetL_Inventory) :!label _label_2)
            (:LoopBody
              (if (== (.RowName (Utilities|Struct|BreakDataTableRowHandle _array_element_2)) (.rowname (.ItemNeeded (Utilities|Struct|BreakS_PuzzleData _array_element))))
                (Class|PuzzleInterface|GiveItemtoPuzzle(Message) (LocalVariables|GetL_HitActor) _array_element_2 _array_index)
                (Utilities|FlowControl|Sequence
                  (:then_0
                    (goto _label_2 Break))
                  (:then_1
                    (goto _label Break)))))))))))