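; GI_KidA is a puzzle-logic Blueprint, apparently the Game Instance, that tracks placed puzzle items and level completion.
; AddItemPlaced flags the given index in the ItemPlaced array and increments LevelsCompleted.
; When the count reaches three it opens the Exterior level; otherwise it prints that item's placed flag.
; The increment happens on every call, without checking whether that index was already set.
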(fn AddItemPlaced
  (params (Index :type Integer))
  (bind _levelscompleted (Variables|Default|GetLevelsCompleted))
  (Utilities|Array|SetArrayElem (Variables|Default|GetItemPlaced) Index true)
  (Math|Integer|IncrementInt _levelscompleted
    (:%20%20
      (if (== _levelscompleted 3)
        (Game|OpenLevel(byName) "Exterior")
        (else
          (Development|PrintString (Utilities|String|ToString(Boolean) (Utilities|Array|Get(acopy) (Variables|Default|GetItemPlaced) Index))))))))