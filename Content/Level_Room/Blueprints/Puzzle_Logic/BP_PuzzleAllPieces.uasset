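; Puzzle actor with three placement points, where item pieces appear as they are placed.
; BeginPlay fills Data with slot transforms, expected Items and false flags, though the third entry reuses the second point's transform.
; PlaceItem calls PlacePieces, which picks the point by index, adds a static mesh component, sets its mesh from the item's data table row and snaps it on.
; Placement neither reads nor updates Data.
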(event EventBeginPlay
  (bind _puzzle1_place (Variables|Default|GetPuzzle1_Place))
  (Utilities|Array|Add (Variables|Default|GetData) (Utilities|Struct|MakeS_PuzzleData _puzzle1_place (Transformation|GetRelativeTransform _puzzle1_place) (Utilities|Array|Get(acopy) (Variables|Default|GetItems)) false))
  (Utilities|Array|Add (Variables|Default|GetData) (Utilities|Struct|MakeS_PuzzleData 0 (Transformation|GetRelativeTransform (Variables|Default|GetPuzzle2_Place)) (Utilities|Array|Get(acopy) (Variables|Default|GetItems) 1) false))
  (Utilities|Array|Add (Variables|Default|GetData) (Utilities|Struct|MakeS_PuzzleData 0 (Transformation|GetRelativeTransform (Variables|Default|GetPuzzle2_Place)) (Utilities|Array|Get(acopy) (Variables|Default|GetItems) 2) false)))

(event EventPlaceItem
  (params (Index :type Integer) (Item :type Data%20Table%20Row%20Handle%20Structure))
  (CallFunction|PlacePieces Index Item))

(fn ConstructionScript
  (|CallParentFunction))

(fn PlacePieces
  (params (Index :type Integer) (Item :type Data%20Table%20Row%20Handle%20Structure))
  (bind (_datatable _rowname) (Utilities|Struct|BreakDataTableRowHandle Item))
  (switch int Index
    (:0
      (LocalVariables|SetL_Component (Variables|Default|GetPuzzle1_Place)))
    (:1
      (LocalVariables|SetL_Component (Variables|Default|GetPuzzle2_Place)))
    (:2
      (LocalVariables|SetL_Component (Variables|Default|GetPuzzle3_Place))))
  (bind _returnvalue (AddComponent|AddStaticMeshComponent false))
  (bind _returnvalue_2 (Utilities|GetDataTableRow _datatable _rowname)
    (:then
      (Components|StaticMesh|SetStaticMesh _returnvalue (.Mesh (Utilities|Struct|BreakS_Inventory _returnvalue_2)))
      (Transformation|AttachComponentToComponent _returnvalue (LocalVariables|GetL_Component) "None" "SnapToTarget" "SnapToTarget" "SnapToTarget" true))))